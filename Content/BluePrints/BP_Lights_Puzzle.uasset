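; Interactable lights puzzle where the player flips four clickable switches to shift two needles.
; Interaction blends the view to the puzzle, shows the cursor and disables movement, while overlap radii toggle its icons.
; Each switch flip-flops a rotation timeline whose finish nudges the needles by fixed offsets and checks the answer.
; Switches 1, 2 and 4 on with 3 off fires the completion call and restores player control.
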(event OnComponentBeginOverlap(OuterIconRadius)
  (params (OverlappedComponent :type Primitive%20Component%20Object%20Reference) (OtherActor :type Actor%20Object%20Reference) (OtherComp :type Primitive%20Component%20Object%20Reference) (OtherBodyIndex :type Integer) (bFromSweep :type Boolean) (SweepResult :type Hit%20Result%20Structure%20%28by%20ref%29))
  (if (== OtherActor (Game|GetPlayerCharacter 0))
    (Development|SetHiddeninGame (Variables|Default|GetOuterIcon) false false)))

(event OnComponentEndOverlap(OuterIconRadius)
  (params (OverlappedComponent :type Primitive%20Component%20Object%20Reference) (OtherActor :type Actor%20Object%20Reference) (OtherComp :type Primitive%20Component%20Object%20Reference) (OtherBodyIndex :type Integer))
  (if (== (Game|GetPlayerCharacter 0) OtherActor)
    (Development|SetHiddeninGame (Variables|Default|GetOuterIcon) true false)))

(event OnComponentBeginOverlap(InnerIconRadius)
  (params (OverlappedComponent :type Primitive%20Component%20Object%20Reference) (OtherActor :type Actor%20Object%20Reference) (OtherComp :type Primitive%20Component%20Object%20Reference) (OtherBodyIndex :type Integer) (bFromSweep :type Boolean) (SweepResult :type Hit%20Result%20Structure%20%28by%20ref%29))
  (if (== OtherActor (Game|GetPlayerCharacter 0))
    (Development|SetHiddeninGame (Variables|Default|GetInnerIcon) false false)
    (Development|SetHiddeninGame (Variables|Default|GetOuterIcon) true false)))

(event OnComponentEndOverlap(InnerIconRadius)
  (params (OverlappedComponent :type Primitive%20Component%20Object%20Reference) (OtherActor :type Actor%20Object%20Reference) (OtherComp :type Primitive%20Component%20Object%20Reference) (OtherBodyIndex :type Integer))
  (if (== (Game|GetPlayerCharacter 0) OtherActor)
    (Development|SetHiddeninGame (Variables|Default|GetInnerIcon) true false)
    (Development|SetHiddeninGame (Variables|Default|GetOuterIcon) false false)))

(event OnClicked(SM_Switch_02)
  (params (TouchedComponent :type Primitive%20Component%20Object%20Reference) (ButtonPressed :type Key%20Structure :default "None"))
  ;[0.15 0.15 0.15 0.5] Move Switches
  (Utilities|FlowControl|FlipFlop
    (:A
      (Variables|Default|SetSwicth_02_On true)
      (Audio|PlaySound2D "/Game/Sounds/SFX_Switch01.SFX_Switch01" 1.0 1.0 0.0 0 0)
      (bind _rotate (Timeline|Timeline Play)
        (:Update
          (Transformation|SetRelativeRotation (Variables|Default|GetSM_Switch_02) (Math|Rotator|MakeRotator 0.0 _rotate 0.0) false false))
        (:Finished
          (CallFunction|Switch02)
          (CallFunction|AnswerCheck))))
    (:B
      (Variables|Default|SetSwicth_02_On false)
      (Audio|PlaySound2D "/Game/Sounds/SFX_Switch02.SFX_Switch02" 1.0 1.0 0.0 0 0)
      (Timeline|Timeline Reverse))))

(event OnClicked(SM_Switch_03)
  (params (TouchedComponent :type Primitive%20Component%20Object%20Reference) (ButtonPressed :type Key%20Structure :default "None"))
  ;[0.15 0.15 0.15 0.5] Move Switches
  (Utilities|FlowControl|FlipFlop
    (:A
      (Variables|Default|SetSwicth_03_On true)
      (Audio|PlaySound2D "/Game/Sounds/SFX_Switch01.SFX_Switch01" 1.0 1.0 0.0 0 0)
      (bind _rotate (Timeline|Timeline_0 Play)
        (:Update
          (Transformation|SetRelativeRotation (Variables|Default|GetSM_Switch_03) (Math|Rotator|MakeRotator 0.0 _rotate 0.0) false false))
        (:Finished
          (CallFunction|Switch03)
          (CallFunction|AnswerCheck))))
    (:B
      (Variables|Default|SetSwicth_03_On false)
      (Audio|PlaySound2D "/Game/Sounds/SFX_Switch02.SFX_Switch02" 1.0 1.0 0.0 0 0)
      (Timeline|Timeline_0 Reverse))))

(event OnClicked(SM_Switch_04)
  (params (TouchedComponent :type Primitive%20Component%20Object%20Reference) (ButtonPressed :type Key%20Structure :default "None"))
  ;[0.15 0.15 0.15 0.5] Move Switches
  (Utilities|FlowControl|FlipFlop
    (:A
      (Variables|Default|SetSwicth_04_On true)
      (Audio|PlaySound2D "/Game/Sounds/SFX_Switch01.SFX_Switch01" 1.0 1.0 0.0 0 0)
      (bind _rotate (Timeline|Timeline_1 Play)
        (:Update
          (Transformation|SetRelativeRotation (Variables|Default|GetSM_Switch_04) (Math|Rotator|MakeRotator 0.0 _rotate 0.0) false false))
        (:Finished
          (CallFunction|Switch04)
          (CallFunction|AnswerCheck))))
    (:B
      (Variables|Default|SetSwicth_04_On false)
      (Audio|PlaySound2D "/Game/Sounds/SFX_Switch02.SFX_Switch02" 1.0 1.0 0.0 0 0)
      (Timeline|Timeline_1 Reverse))))

(event OnClicked(SM_Switch_01)
  (params (TouchedComponent :type Primitive%20Component%20Object%20Reference) (ButtonPressed :type Key%20Structure :default "None"))
  ;[0.15 0.15 0.15 0.5] Move Switches
  (Utilities|FlowControl|FlipFlop
    (:A
      (Variables|Default|SetSwicth_01_On true)
      (Audio|PlaySound2D "/Game/Sounds/SFX_Switch01.SFX_Switch01" 1.0 1.0 0.0 0 0)
      (bind _rotate (Timeline|Rotate%20Switch Play)
        (:Update
          (Transformation|SetRelativeRotation (Variables|Default|GetSM_Switch_01) (Math|Rotator|MakeRotator 0.0 _rotate 0.0) false false))
        (:Finished
          (CallFunction|Switch01)
          (CallFunction|AnswerCheck))))
    (:B
      (Variables|Default|SetSwicth_01_On false)
      (Audio|PlaySound2D "/Game/Sounds/SFX_Switch02.SFX_Switch02" 1.0 1.0 0.0 0 0)
      (Timeline|Rotate%20Switch Reverse))))

(event Custom|Switch01
  (bind _sm_needle_01 (Variables|Default|GetSM_Needle_01))
  (bind _sm_needle_01_2 (Variables|Default|GetSM_Needle_01))
  (bind _sm_needle_02 (Variables|Default|GetSM_Needle_02))
  (bind _sm_needle_02_2 (Variables|Default|GetSM_Needle_02))
  ;[0.15 0.15 0.15 0.5] Move Needles
  (if (Variables|Default|GetSwicth_01_On)
    (Utilities|FlowControl|Sequence
      (:then_0
        (Components|MoveComponentTo _sm_needle_01 (Variables|/Script/Engine.SceneComponent|GetRelativeLocation _sm_needle_01) (Math|Rotator|MakeRotator (- (.roll (Variables|Default|GetNeedle01%20Rotation)) 2e+01) 0.0 0.0) false false 0.2 false)
        (Variables|Default|SetNeedle01%20Rotation (Math|Rotator|MakeRotator (- (.roll (Variables|Default|GetNeedle01%20Rotation)) 2e+01) 0.0 0.0)))
      (:then_1
        (Components|MoveComponentTo _sm_needle_02 (Variables|/Script/Engine.SceneComponent|GetRelativeLocation _sm_needle_02) (Math|Rotator|MakeRotator (- (.roll (Variables|Default|GetNeedle02%20Rotation)) 1e+01) 0.0 0.0) false false 0.2 false)
        (Variables|Default|SetNeedle02%20Rotation (Math|Rotator|MakeRotator (- (.roll (Variables|Default|GetNeedle02%20Rotation)) 1e+01) 0.0 0.0))))
    (else
      (Utilities|FlowControl|Sequence
        (:then_0
          (Components|MoveComponentTo _sm_needle_01_2 (Variables|/Script/Engine.SceneComponent|GetRelativeLocation _sm_needle_01_2) (Math|Rotator|MakeRotator (- (.roll (Variables|Default|GetNeedle01%20Rotation)) -2e+01) 0.0 0.0) false false 0.2 false)
          (Variables|Default|SetNeedle01%20Rotation (Math|Rotator|MakeRotator (- (.roll (Variables|Default|GetNeedle01%20Rotation)) -2e+01) 0.0 0.0)))
        (:then_1
          (Components|MoveComponentTo _sm_needle_02_2 (Variables|/Script/Engine.SceneComponent|GetRelativeLocation _sm_needle_02_2) (Math|Rotator|MakeRotator (- (.roll (Variables|Default|GetNeedle02%20Rotation)) -1e+01) 0.0 0.0) false false 0.2 false)
          (Variables|Default|SetNeedle02%20Rotation (Math|Rotator|MakeRotator (- (.roll (Variables|Default|GetNeedle02%20Rotation)) -1e+01) 0.0 0.0)))))))

(event Custom|AnswerCheck
  (bind _returnvalue (Game|GetPlayerController 0))
  (bind _playerref (Variables|Default|GetPlayerRef))
  ;[0.15 0.15 0.15 0.5] Check Puzzle Answer
  (if (Math|Boolean|ANDBoolean (Variables|Default|GetSwicth_01_On) (Variables|Default|GetSwicth_02_On) (Variables|Default|GetSwicth_04_On))
    (if (not (Variables|Default|GetSwicth_03_On))
      (Default|CallEVDPuzzleCompleted)
      ;[0.15 0.15 0.15 0.5] Interaction
      (Input|ResetIgnoreLookInput _returnvalue)
      (Game|Player|SetViewTargetwithBlend _returnvalue (Variables|Default|GetPlayerRef) 0.5 "VTBlend_Linear" 0.0 false)
      (Variables|/Script/Engine.PlayerController|SetbEnableClickEvents _returnvalue false)
      (Variables|/Script/Engine.PlayerController|SetbShowMouseCursor _returnvalue false)
      (Pawn|Components|CharacterMovement|SetMovementMode (Variables|/Script/Engine.Character|GetCharacterMovement _playerref) "MOVE_Walking" 0)
      (Default|Initialize _playerref)
      (Rendering|SetVisibility (Variables|Default|GetInnerIcon) true false)
      (Rendering|SetVisibility (Variables|Default|GetTagWidget) false false))))

(event Custom|Switch02
  (bind _sm_needle_01 (Variables|Default|GetSM_Needle_01))
  (bind _sm_needle_01_2 (Variables|Default|GetSM_Needle_01))
  (bind _sm_needle_02 (Variables|Default|GetSM_Needle_02))
  (bind _sm_needle_02_2 (Variables|Default|GetSM_Needle_02))
  ;[0.15 0.15 0.15 0.5] Move Needles
  (if (Variables|Default|GetSwicth_02_On)
    (Utilities|FlowControl|Sequence
      (:then_0
        (Components|MoveComponentTo _sm_needle_01 (Variables|/Script/Engine.SceneComponent|GetRelativeLocation _sm_needle_01) (Math|Rotator|MakeRotator (- (.roll (Variables|Default|GetNeedle01%20Rotation)) 15.0) 0.0 0.0) false false 0.2 false)
        (Variables|Default|SetNeedle01%20Rotation (Math|Rotator|MakeRotator (- (.roll (Variables|Default|GetNeedle01%20Rotation)) 15.0) 0.0 0.0)))
      (:then_1
        (Components|MoveComponentTo _sm_needle_02 (Variables|/Script/Engine.SceneComponent|GetRelativeLocation _sm_needle_02) (Math|Rotator|MakeRotator (- (.roll (Variables|Default|GetNeedle02%20Rotation)) 17.0) 0.0 0.0) false false 0.2 false)
        (Variables|Default|SetNeedle02%20Rotation (Math|Rotator|MakeRotator (- (.roll (Variables|Default|GetNeedle02%20Rotation)) 17.0) 0.0 0.0))))
    (else
      (Utilities|FlowControl|Sequence
        (:then_0
          (Components|MoveComponentTo _sm_needle_01_2 (Variables|/Script/Engine.SceneComponent|GetRelativeLocation _sm_needle_01_2) (Math|Rotator|MakeRotator (- (.roll (Variables|Default|GetNeedle01%20Rotation)) -15.0) 0.0 0.0) false false 0.2 false)
          (Variables|Default|SetNeedle01%20Rotation (Math|Rotator|MakeRotator (- (.roll (Variables|Default|GetNeedle01%20Rotation)) -15.0) 0.0 0.0)))
        (:then_1
          (Components|MoveComponentTo _sm_needle_02_2 (Variables|/Script/Engine.SceneComponent|GetRelativeLocation _sm_needle_02_2) (Math|Rotator|MakeRotator (- (.roll (Variables|Default|GetNeedle02%20Rotation)) -17.0) 0.0 0.0) false false 0.2 false)
          (Variables|Default|SetNeedle02%20Rotation (Math|Rotator|MakeRotator (- (.roll (Variables|Default|GetNeedle02%20Rotation)) -17.0) 0.0 0.0)))))))

(event Custom|Switch03
  (bind _sm_needle_01 (Variables|Default|GetSM_Needle_01))
  (bind _sm_needle_01_2 (Variables|Default|GetSM_Needle_01))
  ;[0.15 0.15 0.15 0.5] Move Needles
  (if (Variables|Default|GetSwicth_03_On)
    (Components|MoveComponentTo _sm_needle_01 (Variables|/Script/Engine.SceneComponent|GetRelativeLocation _sm_needle_01) (Math|Rotator|MakeRotator (- (.roll (Variables|Default|GetNeedle01%20Rotation)) 25.0) 0.0 0.0) false false 0.2 false)
    (Variables|Default|SetNeedle01%20Rotation (Math|Rotator|MakeRotator (- (.roll (Variables|Default|GetNeedle01%20Rotation)) 25.0) 0.0 0.0))
    (else
      (Components|MoveComponentTo _sm_needle_01_2 (Variables|/Script/Engine.SceneComponent|GetRelativeLocation _sm_needle_01_2) (Math|Rotator|MakeRotator (- (.roll (Variables|Default|GetNeedle01%20Rotation)) -25.0) 0.0 0.0) false false 0.2 false)
      (Variables|Default|SetNeedle01%20Rotation (Math|Rotator|MakeRotator (- (.roll (Variables|Default|GetNeedle01%20Rotation)) -25.0) 0.0 0.0)))))

(event Custom|Switch04
  (bind _sm_needle_01 (Variables|Default|GetSM_Needle_01))
  (bind _sm_needle_01_2 (Variables|Default|GetSM_Needle_01))
  (bind _sm_needle_02 (Variables|Default|GetSM_Needle_02))
  (bind _sm_needle_02_2 (Variables|Default|GetSM_Needle_02))
  ;[0.15 0.15 0.15 0.5] Move Needles
  (if (Variables|Default|GetSwicth_04_On)
    (Utilities|FlowControl|Sequence
      (:then_0
        (Components|MoveComponentTo _sm_needle_01_2 (Variables|/Script/Engine.SceneComponent|GetRelativeLocation _sm_needle_01_2) (Math|Rotator|MakeRotator (- (.roll (Variables|Default|GetNeedle01%20Rotation)) -5.0) 0.0 0.0) false false 0.2 false)
        (Variables|Default|SetNeedle01%20Rotation (Math|Rotator|MakeRotator (- (.roll (Variables|Default|GetNeedle01%20Rotation)) -5.0) 0.0 0.0)))
      (:then_1
        (Components|MoveComponentTo _sm_needle_02_2 (Variables|/Script/Engine.SceneComponent|GetRelativeLocation _sm_needle_02_2) (Math|Rotator|MakeRotator (- (.roll (Variables|Default|GetNeedle02%20Rotation)) 23.0) 0.0 0.0) false false 0.2 false)
        (Variables|Default|SetNeedle02%20Rotation (Math|Rotator|MakeRotator (- (.roll (Variables|Default|GetNeedle02%20Rotation)) 23.0) 0.0 0.0))))
    (else
      (Utilities|FlowControl|Sequence
        (:then_0
          (Components|MoveComponentTo _sm_needle_01 (Variables|/Script/Engine.SceneComponent|GetRelativeLocation _sm_needle_01) (Math|Rotator|MakeRotator (- (.roll (Variables|Default|GetNeedle01%20Rotation)) 5.0) 0.0 0.0) false false 0.2 false)
          (Variables|Default|SetNeedle01%20Rotation (Math|Rotator|MakeRotator (- (.roll (Variables|Default|GetNeedle01%20Rotation)) 5.0) 0.0 0.0)))
        (:then_1
          (Components|MoveComponentTo _sm_needle_02 (Variables|/Script/Engine.SceneComponent|GetRelativeLocation _sm_needle_02) (Math|Rotator|MakeRotator (- (.roll (Variables|Default|GetNeedle02%20Rotation)) -23.0) 0.0 0.0) false false 0.2 false)
          (Variables|Default|SetNeedle02%20Rotation (Math|Rotator|MakeRotator (- (.roll (Variables|Default|GetNeedle02%20Rotation)) -23.0) 0.0 0.0)))))))

(event Input|EnhancedActionEvents|EnhancedInputActionIA_Back
  (params (ActionValue :type Vector%202D%20Structure) (ElapsedSeconds :type Float%20%28double-precision%29) (TriggeredSeconds :type Float%20%28double-precision%29) (InputAction :type Input%20Action%20Object%20Reference :default "/Game/Input/Actions/IA_Back.IA_Back")))

(event EventBeginPlay
  ;[0.15 0.15 0.15 0.5] Assign Player Input and Needle rotation
  (|CallParentFunction)
  (Input|EnableInput (Game|GetPlayerController 0))
  (Variables|Default|SetNeedle01%20Rotation (Variables|/Script/Engine.SceneComponent|GetRelativeRotation (Variables|Default|GetSM_Needle_01)))
  (Variables|Default|SetNeedle02%20Rotation (Variables|/Script/Engine.SceneComponent|GetRelativeRotation (Variables|Default|GetSM_Needle_02))))

(event EventInteraction
  (bind _returnvalue (Game|GetPlayerController 0))
  (bind _playerref (Variables|Default|GetPlayerRef))
  ;[0.15 0.15 0.15 0.5] Interaction
  (Input|SetIgnoreLookInput _returnvalue true)
  (Game|Player|SetViewTargetwithBlend _returnvalue self 0.5 "VTBlend_Linear" 0.0 false)
  (Variables|/Script/Engine.PlayerController|SetbEnableClickEvents _returnvalue true)
  (Variables|/Script/Engine.PlayerController|SetbShowMouseCursor _returnvalue true)
  (Pawn|Components|CharacterMovement|DisableMovement (Variables|/Script/Engine.Character|GetCharacterMovement _playerref))
  (Default|RemoveHud _playerref)
  (Rendering|SetVisibility (Variables|Default|GetInnerIcon) false false))

(fn ConstructionScript
  (|CallParentFunction)
  (Transformation|SetWorldScale3D (Variables|Default|GetInnerIcon) (Math|Conversions|ToVector(Float) (/ (Variables|Default|GetIconSize) 1e+01)))
  (Transformation|SetRelativeLocation (Variables|Default|GetInnerIcon) (Variables|Default|GetIconLocation) false false))