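; BP_Cup_Pickup is a rubbish cup interactable, labelled "Clean Up Rubbish", that the player can clean up after talking to the moth.
; A looping timer polls BP_Moth_Dialogue until its interacted flag enables the task.
; Interaction then waits briefly, plays a sound, destroys the cup and stops and resets the WBP_HUD clock.
; Two overlap radii swap outer and inner proximity icons, which the construction script sizes and positions.
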(event OnComponentBeginOverlap(InnerIconRadius)
  (params (OverlappedComponent :type Primitive%20Component%20Object%20Reference) (OtherActor :type Actor%20Object%20Reference) (OtherComp :type Primitive%20Component%20Object%20Reference) (OtherBodyIndex :type Integer) (bFromSweep :type Boolean) (SweepResult :type Hit%20Result%20Structure%20%28by%20ref%29))
  ;[0.15 0.15 0.15 0.5] Displaying Inner and Outer Icons
  (if (== OtherActor (Game|GetPlayerCharacter 0))
    (Development|SetHiddeninGame (Variables|Default|GetInnerIcon) false false)
    (Development|SetHiddeninGame (Variables|Default|GetOuterIcon) true false)))

(event OnComponentEndOverlap(InnerIconRadius)
  (params (OverlappedComponent :type Primitive%20Component%20Object%20Reference) (OtherActor :type Actor%20Object%20Reference) (OtherComp :type Primitive%20Component%20Object%20Reference) (OtherBodyIndex :type Integer))
  ;[0.15 0.15 0.15 0.5] Displaying Inner and Outer Icons
  (if (== (Game|GetPlayerCharacter 0) OtherActor)
    (Development|SetHiddeninGame (Variables|Default|GetInnerIcon) true false)
    (Development|SetHiddeninGame (Variables|Default|GetOuterIcon) false false)))

(event OnComponentBeginOverlap(OuterIconRadius)
  (params (OverlappedComponent :type Primitive%20Component%20Object%20Reference) (OtherActor :type Actor%20Object%20Reference) (OtherComp :type Primitive%20Component%20Object%20Reference) (OtherBodyIndex :type Integer) (bFromSweep :type Boolean) (SweepResult :type Hit%20Result%20Structure%20%28by%20ref%29))
  ;[0.15 0.15 0.15 0.5] Displaying Inner and Outer Icons
  (if (== OtherActor (Game|GetPlayerCharacter 0))
    (Development|SetHiddeninGame (Variables|Default|GetOuterIcon) false false)))

(event OnComponentEndOverlap(OuterIconRadius)
  (params (OverlappedComponent :type Primitive%20Component%20Object%20Reference) (OtherActor :type Actor%20Object%20Reference) (OtherComp :type Primitive%20Component%20Object%20Reference) (OtherBodyIndex :type Integer))
  ;[0.15 0.15 0.15 0.5] Displaying Inner and Outer Icons
  (if (== (Game|GetPlayerCharacter 0) OtherActor)
    (Development|SetHiddeninGame (Variables|Default|GetOuterIcon) true false)))

(event Custom|Task%20Started
  (bind _returnvalue (Actor|GetActorOfClass "/Game/BluePrints/Dialogue/BP_Moth_Dialogue.BP_Moth_Dialogue_C"))
  (bind _asbp_moth_dialogue (Utilities|Casting|CastToBP_Moth_Dialogue _returnvalue))
  (if (Variables|/Game/BluePrints/Dialogue/BP_Moth_Dialogue.BP_Moth_Dialogue_C|GetInteracted%20with%20Moth _asbp_moth_dialogue)
    (Variables|Default|SetTaskCanStart true)))

(event EventBeginPlay
  (Utilities|Time|SetTimerbyEvent (delegate Custom|Task%20Started) 0.25 true))

(event EventInteraction
  (if (Variables|Default|GetTaskCanStart)
    (Utilities|FlowControl|Delay 0.2)
    (Audio|PlaySound2D "/Game/Sounds/SFX_Rubbish.SFX_Rubbish" 1.0 1.0 0.0 0 0)
    (Actor|DestroyActor)
    (Utilities|FlowControl|DoOnce false
      (:Completed
        (bind _foundwidgets (Widget|GetAllWidgetsOfClass "/Game/Widget/WBP_HUD.WBP_HUD_C" true))
        (Default|StopandResetClock (Utilities|Array|Get(acopy) _foundwidgets))))))

(fn ConstructionScript
  (Transformation|SetWorldScale3D (Variables|Default|GetInnerIcon) (Math|Conversions|ToVector(Float) (/ (Variables|Default|GetIconSize) 1e+01)))
  (Transformation|SetRelativeLocation (Variables|Default|GetInnerIcon) (Variables|Default|GetIconLocation) false false))

(fn SendOutNotification
  (params (Component :type Primitive%20Component%20Object%20Reference))
  (return "Clean Up Rubbish"))