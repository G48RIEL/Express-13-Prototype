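; Interactable furnace where the player places coal, with proximity icons and a text prompt.
; Interaction checks the character's GotCoal, clears GotCoalText and calls CallEVDCoalPlace; a looping timer polls that flag to show AddedCoal and hide the tag widget.
; Inner and outer overlap volumes swap icons, which the construction script scales and positions.
; SendOutNotification returns the place-coal text until coal is placed, then the no-coal text.
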(event OnComponentBeginOverlap(OuterIconRadius)
  (params (OverlappedComponent :type Primitive%20Component%20Object%20Reference) (OtherActor :type Actor%20Object%20Reference) (OtherComp :type Primitive%20Component%20Object%20Reference) (OtherBodyIndex :type Integer) (bFromSweep :type Boolean) (SweepResult :type Hit%20Result%20Structure%20%28by%20ref%29))
  ;[0.15 0.15 0.15 0.5] Furnace Radius Icons
  (if (== OtherActor (Game|GetPlayerCharacter 0))
    (Development|SetHiddeninGame (Variables|Default|GetOuterIcon) false false)))

(event OnComponentEndOverlap(OuterIconRadius)
  (params (OverlappedComponent :type Primitive%20Component%20Object%20Reference) (OtherActor :type Actor%20Object%20Reference) (OtherComp :type Primitive%20Component%20Object%20Reference) (OtherBodyIndex :type Integer))
  ;[0.15 0.15 0.15 0.5] Furnace Radius Icons
  (if (== (Game|GetPlayerCharacter 0) OtherActor)
    (Development|SetHiddeninGame (Variables|Default|GetOuterIcon) true false)))

(event OnComponentBeginOverlap(InnerIconRadius)
  (params (OverlappedComponent :type Primitive%20Component%20Object%20Reference) (OtherActor :type Actor%20Object%20Reference) (OtherComp :type Primitive%20Component%20Object%20Reference) (OtherBodyIndex :type Integer) (bFromSweep :type Boolean) (SweepResult :type Hit%20Result%20Structure%20%28by%20ref%29))
  ;[0.15 0.15 0.15 0.5] Furnace Radius Icons
  (if (== OtherActor (Game|GetPlayerCharacter 0))
    (Development|SetHiddeninGame (Variables|Default|GetInnerIcon) false false)
    (Development|SetHiddeninGame (Variables|Default|GetOuterIcon) true false)))

(event OnComponentEndOverlap(InnerIconRadius)
  (params (OverlappedComponent :type Primitive%20Component%20Object%20Reference) (OtherActor :type Actor%20Object%20Reference) (OtherComp :type Primitive%20Component%20Object%20Reference) (OtherBodyIndex :type Integer))
  ;[0.15 0.15 0.15 0.5] Furnace Radius Icons
  (if (== (Game|GetPlayerCharacter 0) OtherActor)
    (Development|SetHiddeninGame (Variables|Default|GetInnerIcon) true false)
    (Development|SetHiddeninGame (Variables|Default|GetOuterIcon) false false)))

(event Custom|Check%20For%20Coal
  ;[0.15 0.15 0.15 0.5] Place Coal
  (if (not (Variables|Default|GetGotCoalText?))
    (Rendering|SetVisibility (Variables|Default|GetAddedCoal) true false)
    ;;[0.15 0.15 0.15 0.5] Coal!!
    (Rendering|SetVisibility (Variables|Default|GetTag_Widget) false false)))

(event EventInteraction
  ;[0.15 0.15 0.15 0.5] Place Coal
  (bind _returnvalue (Actor|GetActorOfClass "/Game/FirstPerson/Blueprints/BP_FirstPersonCharacter.BP_FirstPersonCharacter_C"))
  (bind _asbp_first_person_character (Utilities|Casting|CastToBP_FirstPersonCharacter _returnvalue))
  (if (Variables|/Game/FirstPerson/Blueprints/BP_FirstPersonCharacter.BP_FirstPersonCharacter_C|GetGotCoal? _asbp_first_person_character)
    (Variables|Default|SetGotCoalText? false)
    (Default|CallEVDCoalPlace)))

(event EventBeginPlay
  ;[0.15 0.15 0.15 0.5] Place Coal
  (Variables|Default|SetGotCoalText? true)
  (Utilities|Time|SetTimerbyFunctionName 0 "Check For Coal" 0.1 true))

(fn ConstructionScript
  (Transformation|SetWorldScale3D (Variables|Default|GetInnerIcon) (Math|Conversions|ToVector(Float) (/ (Variables|Default|GetIconSize) 1e+01)))
  (Transformation|SetRelativeLocation (Variables|Default|GetInnerIcon) (Variables|Default|GetIconLocation) false false))

(fn SendOutNotification
  (params (Component :type Primitive%20Component%20Object%20Reference))
  (return (select (Variables|Default|GetGotCoalText?) (Variables|Default|GetPlaceCoalText) (Variables|Default|GetNoCoalText))))