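; BP_Food_Pickup is an interactable food pickup for a task tied to interacting with BP_Snake_Dialogue.
; A looping quarter-second timer mirrors the snake's InteractedWithSnake flag into TaskCanStart, which gates Interaction.
; Interacting briefly delays, hides the food, fires the FoodCollected dispatcher, clears the snake flag and resets the HUD clock, then restores visibility after a delay.
; SendOutNotification supplies the "Pick Up Food" prompt.
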(event Custom|Task%20Started
  (bind _returnvalue (Actor|GetActorOfClass "/Game/BluePrints/Dialogue/BP_Snake_Dialogue.BP_Snake_Dialogue_C"))
  (bind _asbp_snake_dialogue (Utilities|Casting|CastToBP_Snake_Dialogue _returnvalue))
  (if (Variables|/Game/BluePrints/Dialogue/BP_Snake_Dialogue.BP_Snake_Dialogue_C|GetInteracted%20With%20Snake _asbp_snake_dialogue)
    (Variables|Default|SetTaskCanStart true)
    (else
      (Variables|Default|SetTaskCanStart false))))

(event EventBeginPlay
  (Utilities|Time|SetTimerbyEvent (delegate Custom|Task%20Started) 0.25 true))

(event EventInteraction
  (if (Variables|Default|GetTaskCanStart)
    (Utilities|FlowControl|Delay 0.2)
    (Rendering|SetVisibility (Variables|Default|GetFood) false false)
    (Default|CallEVDFoodCollected)
    (bind _returnvalue (Actor|GetActorOfClass "/Game/BluePrints/Dialogue/BP_Snake_Dialogue.BP_Snake_Dialogue_C"))
    (bind _asbp_snake_dialogue (Utilities|Casting|CastToBP_Snake_Dialogue _returnvalue))
    (Variables|/Game/BluePrints/Dialogue/BP_Snake_Dialogue.BP_Snake_Dialogue_C|SetInteracted%20With%20Snake _asbp_snake_dialogue false)
    (bind _foundwidgets (Widget|GetAllWidgetsOfClass "/Game/Widget/WBP_HUD.WBP_HUD_C" true))
    (Default|StopandResetClock (Utilities|Array|Get(acopy) _foundwidgets))
    (Utilities|FlowControl|Delay 5.0)
    (Rendering|SetVisibility (Variables|Default|GetFood) true false)))

(fn ConstructionScript)

(fn SendOutNotification
  (params (Component :type Primitive%20Component%20Object%20Reference))
  (return "Pick Up Food"))