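; Interactable door that swings open through a half turn and supplies an "Open Door" prompt.
; Interaction plays a Timeline that lerps the hinge yaw from StartingLocation and flags DoorOpen, with no closing logic.
; Two overlap radii swap outer and inner icons as the player approaches, hiding both on overlap changes once open.
; The construction script scales and positions both icons from IconSize and IconLocation.
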(event OnComponentBeginOverlap(InnerIconRadius)
  (params (OverlappedComponent :type Primitive%20Component%20Object%20Reference) (OtherActor :type Actor%20Object%20Reference) (OtherComp :type Primitive%20Component%20Object%20Reference) (OtherBodyIndex :type Integer) (bFromSweep :type Boolean) (SweepResult :type Hit%20Result%20Structure%20%28by%20ref%29))
  ;[0.15 0.15 0.15 0.5] Displaying Inner and Outer Icons
  (if (== OtherActor (Game|GetPlayerCharacter 0))
    (Development|SetHiddeninGame (Variables|Default|GetInnerIcon) false false)
    (Development|SetHiddeninGame (Variables|Default|GetOuterIcon) true false)
    (if (Variables|Default|GetDoorOpen?)
      (Development|SetHiddeninGame (Variables|Default|GetInnerIcon) true false))))

(event OnComponentEndOverlap(InnerIconRadius)
  (params (OverlappedComponent :type Primitive%20Component%20Object%20Reference) (OtherActor :type Actor%20Object%20Reference) (OtherComp :type Primitive%20Component%20Object%20Reference) (OtherBodyIndex :type Integer))
  ;[0.15 0.15 0.15 0.5] Displaying Inner and Outer Icons
  (if (== (Game|GetPlayerCharacter 0) OtherActor)
    (Development|SetHiddeninGame (Variables|Default|GetInnerIcon) true false)
    (Development|SetHiddeninGame (Variables|Default|GetOuterIcon) false false)
    (if (Variables|Default|GetDoorOpen?)
      (Development|SetHiddeninGame (Variables|Default|GetInnerIcon) true false))))

(event OnComponentBeginOverlap(OuterIconRadius)
  (params (OverlappedComponent :type Primitive%20Component%20Object%20Reference) (OtherActor :type Actor%20Object%20Reference) (OtherComp :type Primitive%20Component%20Object%20Reference) (OtherBodyIndex :type Integer) (bFromSweep :type Boolean) (SweepResult :type Hit%20Result%20Structure%20%28by%20ref%29))
  ;[0.15 0.15 0.15 0.5] Displaying Inner and Outer Icons
  (if (== OtherActor (Game|GetPlayerCharacter 0))
    (Development|SetHiddeninGame (Variables|Default|GetOuterIcon) false false)
    (if (Variables|Default|GetDoorOpen?)
      (Development|SetHiddeninGame (Variables|Default|GetInnerIcon) true false))))

(event OnComponentEndOverlap(OuterIconRadius)
  (params (OverlappedComponent :type Primitive%20Component%20Object%20Reference) (OtherActor :type Actor%20Object%20Reference) (OtherComp :type Primitive%20Component%20Object%20Reference) (OtherBodyIndex :type Integer))
  ;[0.15 0.15 0.15 0.5] Displaying Inner and Outer Icons
  (if (== (Game|GetPlayerCharacter 0) OtherActor)
    (Development|SetHiddeninGame (Variables|Default|GetOuterIcon) true false)
    (if (Variables|Default|GetDoorOpen?)
      (Development|SetHiddeninGame (Variables|Default|GetInnerIcon) true false))))

(event EventInteraction
  (bind _startinglocation (Variables|Default|GetStartingLocation))
  (bind _rotate (Timeline|Timeline Play)
    (:Update
      (Transformation|SetRelativeRotation (Variables|Default|Getdoor_hinge) (Math|Rotator|MakeRotator 0.0 0.0 (Math|Float|Lerp (.yaw _startinglocation) (- (.yaw _startinglocation) 1.8e+02) _rotate)) false false)
      (Variables|Default|SetDoorOpen? true))))

(fn ConstructionScript
  (Transformation|SetWorldScale3D (Variables|Default|GetInnerIcon) (Math|Conversions|ToVector(Float) (/ (Variables|Default|GetIconSize) 1e+01)))
  (Transformation|SetRelativeLocation (Variables|Default|GetInnerIcon) (Variables|Default|GetIconLocation) false false))

(fn SendOutNotification
  (params (Component :type Primitive%20Component%20Object%20Reference))
  (return "Open Door"))