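; Dialogue component, going by its BPC prefix, that steps through an array of lines, pausing the game while they show.
; It creates a W_Dialogue widget at BeginPlay.
; Each Speech call sends the current line, speaker name, text delay and Customer value to the widget, then advances the index.
; The call after the last line resets the index, clears the widget and unpauses.
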(event Custom|Speech
  (bind _dialogue (Variables|Default|GetDialogue))
  (Game|SetGamePaused true)
  (Default|IncomingText (Variables|Default|GetW_DialougeRef) (Utilities|Array|Get(acopy) _dialogue (Variables|Default|GetCurrentDialogue)) (Variables|Default|GetTextDelay) (Variables|Default|GetName) (Variables|Default|GetCustomer))
  (bind _result (Math|Integer|IncrementInt (Variables|Default|GetCurrentDialogue))
    (:%20%20
      (if (>= _result (+ (Utilities|Array|Length _dialogue) 1))
        (Variables|Default|SetCurrentDialogue 0)
        (Default|ClearScreen (Variables|Default|GetW_DialougeRef))
        (Game|SetGamePaused false)))))

(event EventBeginPlay
  (bind _returnvalue (UserInterface|CreateWidget "/Game/Widget/W_Dialogue.W_Dialogue_C"))
  (Variables|Default|SetW_DialougeRef _returnvalue))