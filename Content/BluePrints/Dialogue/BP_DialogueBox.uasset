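; BP_DialogueBox is an interactable dialogue actor that plays speech and passes a tag marker on to a next customer.
; On Interaction it triggers Speech on its BPCDialogue component and hides its TagWidget.
; It then picks a random BP_DialogueBox from all those in the level, possibly itself, as NextCustomer and shows that actor's TagWidget.
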(event EventInteraction
  (Default|Speech (Variables|Default|GetBPC_Dialogue))
  (Rendering|SetVisibility (Variables|Default|GetTagWidget) false false)
  (bind _outactors (Actor|GetAllActorsOfClass "BP_DialogueBox_C"))
  (Variables|Default|SetNextCustomer (Utilities|Array|Get(acopy) _outactors (Math|Random|RandomInteger (Utilities|Array|Length _outactors))))
  (bind _nextcustomer (Variables|Default|GetNextCustomer)
    (:then
      (Rendering|SetVisibility (Variables|BP_DialogueBox_C|GetTagWidget _nextcustomer) true false))
    (:else)))

(fn ConstructionScript)