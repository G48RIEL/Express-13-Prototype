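; BP_Human_Dialogue2 is an interactable human that starts dialogue and passes a tag marker on to a random next customer.
; On Interaction it flags Human 2 as interacted with, triggers Speech on its dialogue component and hides its own tag widget.
; It then picks a random BP_DialogueBox actor in the level as NextCustomer and, if valid, shows that actor's tag widget.
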(event EventInteraction
  (Variables|Default|SetInteracted%20with%20human%202 true)
  (Default|Speech (Variables|Default|GetBPC_Dialogue))
  (Rendering|SetVisibility (Variables|Default|GetTagWidget) false false)
  (bind _outactors (Actor|GetAllActorsOfClass "/Game/BluePrints/Dialogue/BP_DialogueBox.BP_DialogueBox_C"))
  (Variables|Default|SetNextCustomer (Utilities|Array|Get(acopy) _outactors (Math|Random|RandomInteger (Utilities|Array|Length _outactors))))
  (bind _nextcustomer (Variables|Default|GetNextCustomer)
    (:then
      (Rendering|SetVisibility (Variables|/Game/BluePrints/Dialogue/BP_DialogueBox.BP_DialogueBox_C|GetTagWidget _nextcustomer) true false))
    (:else)))

(fn ConstructionScript
  (|CallParentFunction))